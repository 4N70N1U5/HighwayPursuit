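; Player car pawn for an obstacle-dodging driving game, with toggleable first- and third-person cameras.
; Tick derives Score from X distance, drives forward even without input and raises movement speed with Score, while clamping sideways steering to the road width.
; Overlapping speed bumps, cones or barriers applies damage; bumps and cones flash the paint red, and cones flatten.
; At zero Health, it refills Health and calls MyGameMode's GameOver with the start location.
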(event `self.ReceiveBeginPlay`
  (set `self.PlayerStartLocation` (`self.K2_GetActorLocation`)))

(event `self.ReceiveTick`
  (params (DeltaSeconds :type "Float (single-precision)"))
  (bind (_returnvalue_x _returnvalue_y _returnvalue_z) (`KismetMathLibrary.BreakVector` (`self.K2_GetActorLocation`)))
  (bind _floatingpawnmovement (`self.FloatingPawnMovement`))
  (bind _returnvalue (`KismetMathLibrary.GetForwardVector` (`KismetMathLibrary.MakeRotator` (.yaw (`self.GetControlRotation`)))))
  ;[1 1 1] Forward movement and speed
  ;[1 1 1] Calculate score
  (bind _output_get (set `self.Score` (`KismetMathLibrary.FTrunc` (/ (+ (.x (.location (`self.GetTransform`))) 7000.0) 1000.0))))
  (if (== (stale `InputAxis|Forward/Backward` AxisValue) 0.0)
    (`self.AddMovementInput` _returnvalue 0.7)
    (else
      (`self.AddMovementInput` _returnvalue (stale `InputAxis|Forward/Backward` AxisValue))))
  (bind _returnvalue_2 (`KismetMathLibrary.Conv_IntToDouble` (+ (* _output_get 10) 20000)))
  ;[1 1 1] Accelerate movement speed
  (set `FloatingPawnMovement.MaxSpeed` _returnvalue_2 _floatingpawnmovement)
  (set `FloatingPawnMovement.Acceleration` _returnvalue_2 _floatingpawnmovement)
  (set `FloatingPawnMovement.Deceleration` _returnvalue_2 _floatingpawnmovement)
  (if (<= _returnvalue_y -2500.0)
    (`self.K2_SetActorLocation` (`KismetMathLibrary.MakeVector` _returnvalue_x -2500.0 _returnvalue_z))
    (elif (>= _returnvalue_y 2500.0)
      (`self.K2_SetActorLocation` (`KismetMathLibrary.MakeVector` _returnvalue_x 2500.0 _returnvalue_z)))))

(event `InputAxis|Forward/Backward`
  (params (AxisValue :type "Float (single-precision)"))
  ;[1 1 1] Forward movement and speed
)

(event `InputAxis|Left/Right`
  (params (AxisValue :type "Float (single-precision)"))
  (bind _returnvalue (`KismetMathLibrary.GetRightVector` (`KismetMathLibrary.MakeRotator` (.yaw (`self.GetControlRotation`)))))
  ;[1 1 1] Left/Right movement
  (if (== AxisValue -1.0)
    (if (>= (.y (.location (`self.GetTransform`))) -2500.0)
      (`self.AddMovementInput` _returnvalue -0.3))
    (elif (== AxisValue 1.0)
      (if (<= (.y (.location (`self.GetTransform`))) 2500.0)
        (`self.AddMovementInput` _returnvalue 0.3)))))

(event `InputAction|ToggleCamera`
  (params (Key :type "Key Structure"))
  ;[1 1 1] Toggle first/third person
  (:`Pressed`
    (`/Engine/EditorBlueprintResources/StandardMacros.FlipFlop`
      (:`A`
        (`ActorComponent.SetActive` (`self.FirstPersonCamera`) true false)
        (`ActorComponent.SetActive` (`self.ThirdPersonCamera`) false false))
      (:`B`
        (`ActorComponent.SetActive` (`self.FirstPersonCamera`) false false)
        (`ActorComponent.SetActive` (`self.ThirdPersonCamera`) true false)))))

(event `self.ReceiveActorBeginOverlap`
  (params (OtherActor :type "Actor Object Reference"))
  (bind _returnvalue (`GameplayStatics.GetObjectClass` OtherActor))
  (bind _muscle_car_pack_car1 (`self.Muscle_Car_Pack_Car1`))
  (bind _muscle_car_pack_car1_2 (`self.Muscle_Car_Pack_Car1`))
  (bind _muscle_car_pack_car1_3 (`self.Muscle_Car_Pack_Car1`))
  ;[1 1 1] Damage system
  (bind _returnvalue_2 (`GameplayStatics.GetActorOfClass` "PlayerCar_C"))
  (if (`KismetMathLibrary.ClassIsChildOf` _returnvalue "/Game/Blueprints/SpeedBump.SpeedBump_C")
    (`GameplayStatics.ApplyDamage` _returnvalue_2 10.0)
    (bind _returnvalue_3 (`PrimitiveComponent.CreateDynamicMaterialInstance` _muscle_car_pack_car1_2 0 "/Game/Materials/M_PlayerCarPaint.M_PlayerCarPaint" "None"))
    (bind _returnvalue_4 (`PrimitiveComponent.CreateDynamicMaterialInstance` _muscle_car_pack_car1_2 1 "/Game/Materials/M_PlayerCarPaint.M_PlayerCarPaint" "None"))
    (`MaterialInstanceDynamic.SetVectorParameterValue` _returnvalue_3 "Color" (struct :`R` 1.0 :`A` 1.0))
    (`MaterialInstanceDynamic.SetVectorParameterValue` _returnvalue_4 "Color" (struct :`R` 1.0 :`A` 1.0))
    (`KismetSystemLibrary.Delay` 0.2)
    (`MaterialInstanceDynamic.SetVectorParameterValue` _returnvalue_3 "Color" (struct :`R` 1.0 :`G` 0.15 :`A` 1.0))
    (`MaterialInstanceDynamic.SetVectorParameterValue` _returnvalue_4 "Color" (struct :`R` 1.0 :`G` 0.15 :`A` 1.0))
    (elif (`KismetMathLibrary.ClassIsChildOf` _returnvalue "/Game/Blueprints/TrafficCones.TrafficCones_C")
      (`GameplayStatics.ApplyDamage` _returnvalue_2 20.0)
      (bind _astraffic_cones (cast `/Game/Blueprints/TrafficCones` OtherActor))
      (`/Game/Blueprints/TrafficCones.DisableCollider` _astraffic_cones)
      (bind (_returnvalue_x _returnvalue_y) (`KismetMathLibrary.BreakVector` (`self.GetActorScale3D` _astraffic_cones)))
      (`self.SetActorScale3D` OtherActor (`KismetMathLibrary.MakeVector` _returnvalue_x _returnvalue_y 0.2))
      (bind _returnvalue_5 (`PrimitiveComponent.CreateDynamicMaterialInstance` _muscle_car_pack_car1_3 0 "/Game/Materials/M_PlayerCarPaint.M_PlayerCarPaint" "None"))
      (bind _returnvalue_6 (`PrimitiveComponent.CreateDynamicMaterialInstance` _muscle_car_pack_car1_3 1 "/Game/Materials/M_PlayerCarPaint.M_PlayerCarPaint" "None"))
      (`MaterialInstanceDynamic.SetVectorParameterValue` _returnvalue_5 "Color" (struct :`R` 1.0 :`A` 1.0))
      (`MaterialInstanceDynamic.SetVectorParameterValue` _returnvalue_6 "Color" (struct :`R` 1.0 :`A` 1.0))
      (`KismetSystemLibrary.Delay` 0.1)
      (`MaterialInstanceDynamic.SetVectorParameterValue` _returnvalue_6 "Color" (struct :`R` 1.0 :`G` 0.15 :`A` 1.0))
      (`MaterialInstanceDynamic.SetVectorParameterValue` _returnvalue_5 "Color" (struct :`R` 1.0 :`G` 0.15 :`A` 1.0))
      (`KismetSystemLibrary.Delay` 0.1)
      (bind _returnvalue_7 (`PrimitiveComponent.CreateDynamicMaterialInstance` _muscle_car_pack_car1 0 "/Game/Materials/M_PlayerCarPaint.M_PlayerCarPaint" "None"))
      (bind _returnvalue_8 (`PrimitiveComponent.CreateDynamicMaterialInstance` _muscle_car_pack_car1 1 "/Game/Materials/M_PlayerCarPaint.M_PlayerCarPaint" "None"))
      (`MaterialInstanceDynamic.SetVectorParameterValue` _returnvalue_7 "Color" (struct :`R` 1.0 :`A` 1.0))
      (`MaterialInstanceDynamic.SetVectorParameterValue` _returnvalue_8 "Color" (struct :`R` 1.0 :`A` 1.0))
      (`KismetSystemLibrary.Delay` 0.2)
      (`MaterialInstanceDynamic.SetVectorParameterValue` _returnvalue_8 "Color" (struct :`R` 1.0 :`G` 0.15 :`A` 1.0))
      (`MaterialInstanceDynamic.SetVectorParameterValue` _returnvalue_7 "Color" (struct :`R` 1.0 :`G` 0.15 :`A` 1.0))
      (elif (`KismetMathLibrary.ClassIsChildOf` _returnvalue "/Game/Blueprints/Barrier.Barrier_C")
        (`GameplayStatics.ApplyDamage` _returnvalue_2 100.0)))))

(event `self.ReceiveAnyDamage`
  (params (Damage :type "Float (single-precision)") (DamageType :type "DamageType Object Reference") (InstigatedBy :type "Controller Object Reference") (DamageCauser :type "Actor Object Reference"))
  ;[1 1 1] Damage system
  (bind _output_get (set `self.Health` (`KismetMathLibrary.FClamp` (- (`self.Health`) Damage) 0.0 100.0)))
  (if (<= _output_get 0.0)
    (set `self.Health` 100.0)
    (bind _asmy_game_mode (cast `/Game/Blueprints/MyGameMode` (`GameplayStatics.GetGameMode`)))
    (`/Game/Blueprints/MyGameMode.GameOver` _asmy_game_mode (`self.PlayerStartLocation`))))

(fn `DamageFeedback`
  (bind _returnvalue (`PrimitiveComponent.CreateDynamicMaterialInstance` (`self.Muscle_Car_Pack_Car1`) 0 "/Game/Materials/M_PlayerCarPaint.M_PlayerCarPaint" "None"))
  (`MaterialInstanceDynamic.SetVectorParameterValue` _returnvalue "Color" (struct :`R` 1.0 :`A` 1.0)))

(fn `UserConstructionScript`)