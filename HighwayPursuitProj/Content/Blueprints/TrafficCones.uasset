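; Traffic cone group actor that varies the look of its six cone meshes each time it is constructed.
; The construction script applies a random yaw offset to each cone, setting its world rotation plus offset as relative rotation.
; It then gives each cone a dynamic material instance with a randomized orange-red Color parameter.
; DisableCollider destroys the DamageCollider component but is not called within this Blueprint, and the event graph is empty.
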(event `self.ReceiveActorBeginOverlap`
  (params (OtherActor :type "Actor Object Reference")))

(fn `DisableCollider`
  (`ActorComponent.K2_DestroyComponent` (`self.DamageCollider`)))

(fn `RotateCones`
  (bind _conehighpolyfbx1 (`self.ConeHighPolyFBX1`))
  (bind _conehighpolyfbx2 (`self.ConeHighPolyFBX2`))
  (bind _conehighpolyfbx3 (`self.ConeHighPolyFBX3`))
  (bind _conehighpolyfbx4 (`self.ConeHighPolyFBX4`))
  (bind _conehighpolyfbx5 (`self.ConeHighPolyFBX5`))
  (bind _conehighpolyfbx (`self.ConeHighPolyFBX`))
  (bind (_returnvalue_roll _returnvalue_pitch _returnvalue_yaw) (`KismetMathLibrary.BreakRotator` (`SceneComponent.K2_GetComponentRotation` _conehighpolyfbx4)))
  (bind (_returnvalue_roll_2 _returnvalue_pitch_2 _returnvalue_yaw_2) (`KismetMathLibrary.BreakRotator` (`SceneComponent.K2_GetComponentRotation` _conehighpolyfbx5)))
  (bind (_returnvalue_roll_3 _returnvalue_pitch_3 _returnvalue_yaw_3) (`KismetMathLibrary.BreakRotator` (`SceneComponent.K2_GetComponentRotation` _conehighpolyfbx1)))
  (bind (_returnvalue_roll_4 _returnvalue_pitch_4 _returnvalue_yaw_4) (`KismetMathLibrary.BreakRotator` (`SceneComponent.K2_GetComponentRotation` _conehighpolyfbx2)))
  (bind (_returnvalue_roll_5 _returnvalue_pitch_5 _returnvalue_yaw_5) (`KismetMathLibrary.BreakRotator` (`SceneComponent.K2_GetComponentRotation` _conehighpolyfbx3)))
  (bind (_returnvalue_roll_6 _returnvalue_pitch_6 _returnvalue_yaw_6) (`KismetMathLibrary.BreakRotator` (`SceneComponent.K2_GetComponentRotation` _conehighpolyfbx)))
  (`SceneComponent.K2_SetRelativeRotation` _conehighpolyfbx1 (`KismetMathLibrary.MakeRotator` _returnvalue_roll_3 _returnvalue_pitch_3 (+ _returnvalue_yaw_3 (`KismetMathLibrary.RandomFloatInRange` -30.0 30.0))) false false)
  (`SceneComponent.K2_SetRelativeRotation` _conehighpolyfbx2 (`KismetMathLibrary.MakeRotator` _returnvalue_roll_4 _returnvalue_pitch_4 (+ _returnvalue_yaw_4 (`KismetMathLibrary.RandomFloatInRange` -30.0 30.0))) false false)
  (`SceneComponent.K2_SetRelativeRotation` _conehighpolyfbx3 (`KismetMathLibrary.MakeRotator` _returnvalue_roll_5 _returnvalue_pitch_5 (+ _returnvalue_yaw_5 (`KismetMathLibrary.RandomFloatInRange` -30.0 30.0))) false false)
  (`SceneComponent.K2_SetRelativeRotation` _conehighpolyfbx4 (`KismetMathLibrary.MakeRotator` _returnvalue_roll _returnvalue_pitch (+ _returnvalue_yaw (`KismetMathLibrary.RandomFloatInRange` -30.0 30.0))) false false)
  (`SceneComponent.K2_SetRelativeRotation` _conehighpolyfbx5 (`KismetMathLibrary.MakeRotator` _returnvalue_roll_2 _returnvalue_pitch_2 (+ _returnvalue_yaw_2 (`KismetMathLibrary.RandomFloatInRange` -30.0 30.0))) false false)
  (`SceneComponent.K2_SetRelativeRotation` _conehighpolyfbx (`KismetMathLibrary.MakeRotator` _returnvalue_roll_6 _returnvalue_pitch_6 (+ _returnvalue_yaw_6 (`KismetMathLibrary.RandomFloatInRange` -30.0 30.0))) false false))

(fn `SetColors`
  (bind _returnvalue (`PrimitiveComponent.CreateDynamicMaterialInstance` (`self.ConeHighPolyFBX`) 0 "/Game/Models/TrafficConeHighPoly/01_-_Default.01_-_Default" "None"))
  (`MaterialInstanceDynamic.SetVectorParameterValue` _returnvalue "Color" (make `LinearColor` 0.8 (`KismetMathLibrary.RandomFloatInRange` 0.1 0.3) 0.0 1.0))
  (bind _returnvalue_2 (`PrimitiveComponent.CreateDynamicMaterialInstance` (`self.ConeHighPolyFBX1`) 0 "/Game/Models/TrafficConeHighPoly/01_-_Default.01_-_Default" "None"))
  (`MaterialInstanceDynamic.SetVectorParameterValue` _returnvalue_2 "Color" (make `LinearColor` 0.8 (`KismetMathLibrary.RandomFloatInRange` 0.1 0.3) 0.0 1.0))
  (bind _returnvalue_3 (`PrimitiveComponent.CreateDynamicMaterialInstance` (`self.ConeHighPolyFBX2`) 0 "/Game/Models/TrafficConeHighPoly/01_-_Default.01_-_Default" "None"))
  (`MaterialInstanceDynamic.SetVectorParameterValue` _returnvalue_3 "Color" (make `LinearColor` 0.8 (`KismetMathLibrary.RandomFloatInRange` 0.1 0.3) 0.0 1.0))
  (bind _returnvalue_4 (`PrimitiveComponent.CreateDynamicMaterialInstance` (`self.ConeHighPolyFBX3`) 0 "/Game/Models/TrafficConeHighPoly/01_-_Default.01_-_Default" "None"))
  (`MaterialInstanceDynamic.SetVectorParameterValue` _returnvalue_4 "Color" (make `LinearColor` 0.8 (`KismetMathLibrary.RandomFloatInRange` 0.1 0.3) 0.0 1.0))
  (bind _returnvalue_5 (`PrimitiveComponent.CreateDynamicMaterialInstance` (`self.ConeHighPolyFBX4`) 0 "/Game/Models/TrafficConeHighPoly/01_-_Default.01_-_Default" "None"))
  (`MaterialInstanceDynamic.SetVectorParameterValue` _returnvalue_5 "Color" (make `LinearColor` 0.8 (`KismetMathLibrary.RandomFloatInRange` 0.1 0.3) 0.0 1.0))
  (bind _returnvalue_6 (`PrimitiveComponent.CreateDynamicMaterialInstance` (`self.ConeHighPolyFBX5`) 0 "/Game/Models/TrafficConeHighPoly/01_-_Default.01_-_Default" "None"))
  (`MaterialInstanceDynamic.SetVectorParameterValue` _returnvalue_6 "Color" (make `LinearColor` 0.8 (`KismetMathLibrary.RandomFloatInRange` 0.1 0.3) 0.0 1.0)))

(fn `UserConstructionScript`
  (`self.RotateCones`)
  (`self.SetColors`))