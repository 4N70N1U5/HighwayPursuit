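; Endless-runner road tile that asks MyGameMode for a new tile and destroys itself when the PlayerCar exits its trigger.
; The construction script adds an obstacle at one of three random lane points and a health item at 1-in-20 odds.
; It also spawns a Path and TrafficCar at independently random traffic points, then starts a Timeline sweeping the car along the spline.
; GetAttachTransform exposes the AttachPoint's world transform.
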(event `self.SpawnNewTrigger.OnComponentEndOverlap`
  (params (OverlappedComponent :type "PrimitiveComponent Object Reference") (OtherActor :type "Actor Object Reference") (OtherComp :type "PrimitiveComponent Object Reference") (OtherBodyIndex :type Integer))
  (cast `/Game/Blueprints/PlayerCar` OtherActor)
  (bind _asmy_game_mode (cast `/Game/Blueprints/MyGameMode` (`GameplayStatics.GetGameMode`)))
  (`/Game/Blueprints/MyGameMode.CreateRoadTileEndless` _asmy_game_mode)
  (`self.K2_DestroyActor`))

(event `StartTrafficMovement`
  (bind _spline (`/Game/Blueprints/Path.Spline` (`self.PathReference`)))
  (bind (_direction _alphavalue) (`Timeline|Timeline`)
    (:`Update`
      (bind _returnvalue_location (`KismetMathLibrary.BreakTransform` (`SplineComponent.GetTransformAtDistanceAlongSpline` _spline (`KismetMathLibrary.Lerp` 0.0 (`SplineComponent.GetSplineLength` _spline) _alphavalue) "World" false)))
      (`self.K2_SetActorLocation` (`self.TrafficCarReference`) _returnvalue_location true false))))

(fn `GetAttachTransform`
  (returns (NewParam :type "Transform Structure"))
  (return (`SceneComponent.K2_GetComponentToWorld` (`self.AttachPoint`))))

(fn `SetSpawnPoints`
  (set `self.SpawnPoints` (`|MakeArray` (`SceneComponent.GetRelativeTransform` (`self.SpawnPointLeft`)) (`SceneComponent.GetRelativeTransform` (`self.SpawnPointCenter`)) (`SceneComponent.GetRelativeTransform` (`self.SpawnPointRight`)))))

(fn `SetTrafficSpawnPoints`
  (set `self.TrafficSpawnPoints` (`|MakeArray` (`SceneComponent.GetRelativeTransform` (`self.TrafficSpawnPointLeft`)) (`SceneComponent.GetRelativeTransform` (`self.TrafficSpawnPointCenter`)) (`SceneComponent.GetRelativeTransform` (`self.TrafficSpawnPointRight`)))))

(fn `SpawnHealthItem`
  (bind _healthitemarea (`self.HealthItemArea`))
  (`AddComponent|NODE_AddChildActorComponent-3` :`RelativeTransform` (`KismetMathLibrary.MakeTransform` (`KismetMathLibrary.RandomPointInBoundingBox` (`SceneComponent.RelativeLocation` _healthitemarea) (`BoxComponent.BoxExtent` _healthitemarea)))))

(fn `SpawnObstacle`
  (bind _returnvalue (`KismetMathLibrary.RandomIntegerInRange` 1 100))
  (bind _output (`|GetArrayItem` (`self.SpawnPoints`) (`KismetMathLibrary.RandomIntegerInRange` 0 2)))
  (if (<= _returnvalue 50)
    (`AddComponent|NODE_AddChildActorComponent-0` :`RelativeTransform` _output)
    (elif (<= _returnvalue 80)
      (`AddComponent|NODE_AddChildActorComponent-1` :`RelativeTransform` _output)
      (else
        (`AddComponent|NODE_AddChildActorComponent-2` :`RelativeTransform` _output)))))

(fn `SpawnTraffic`
  (bind _output (`|GetArrayItem` (`self.TrafficSpawnPoints`) (`KismetMathLibrary.RandomIntegerInRange` 0 2)))
  (bind _returnvalue (`|SpawnActorFromClass` "/Game/Blueprints/Path.Path_C" _output "Undefined" "MultiplyWithRoot" null null))
  (set `self.PathReference` _returnvalue)
  (bind _returnvalue_2 (`|SpawnActorFromClass` "/Game/Blueprints/TrafficCar.TrafficCar_C" _output "Undefined" "MultiplyWithRoot" null null))
  (set `self.TrafficCarReference` _returnvalue_2))

(fn `UserConstructionScript`
  (`self.SetSpawnPoints`)
  (`self.SpawnObstacle`)
  (`self.SetTrafficSpawnPoints`)
  (`self.SpawnTraffic`)
  (`self.StartTrafficMovement`)
  (if (== (`KismetMathLibrary.RandomIntegerInRange` 1 20) 1)
    (`self.SpawnHealthItem`)))