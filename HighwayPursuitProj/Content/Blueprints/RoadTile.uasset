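; RoadTile is a road segment actor for an endless driving game with three spawn points.
; The construction script caches left, center and right transforms, then adds one child actor at a random one, choosing among three weighted random branches.
; When PlayerCar leaves SpawnNewTrigger, the tile asks MyGameMode to create a new tile and destroys itself.
; GetAttachTransform exposes the AttachPoint world transform.
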(event `self.SpawnNewTrigger.OnComponentEndOverlap`
  (params (OverlappedComponent :type "PrimitiveComponent Object Reference") (OtherActor :type "Actor Object Reference") (OtherComp :type "PrimitiveComponent Object Reference") (OtherBodyIndex :type Integer))
  (cast `/Game/Blueprints/PlayerCar` OtherActor)
  (bind _asmy_game_mode (cast `/Game/Blueprints/MyGameMode` (`GameplayStatics.GetGameMode`)))
  (`/Game/Blueprints/MyGameMode.CreateRoadTile` _asmy_game_mode)
  (`self.K2_DestroyActor`))

(fn `GetAttachTransform`
  (returns (NewParam :type "Transform Structure"))
  (return (`SceneComponent.K2_GetComponentToWorld` (`self.AttachPoint`))))

(fn `SetSpawnPoints`
  (set `self.SpawnPoints` (`|MakeArray` (`SceneComponent.GetRelativeTransform` (`self.SpawnPointLeft`)) (`SceneComponent.GetRelativeTransform` (`self.SpawnPointCenter`)) (`SceneComponent.GetRelativeTransform` (`self.SpawnPoint Right`)))))

(fn `SpawnObstacle`
  (bind _returnvalue (`KismetMathLibrary.RandomIntegerInRange` 1 100))
  (bind _output (`|GetArrayItem` (`self.SpawnPoints`) (`KismetMathLibrary.RandomIntegerInRange` 0 2)))
  (if (<= _returnvalue 50)
    (`AddComponent|NODE_AddChildActorComponent-0` :`RelativeTransform` _output)
    (elif (<= _returnvalue 80)
      (`AddComponent|NODE_AddChildActorComponent-1` :`RelativeTransform` _output)
      (else
        (`AddComponent|NODE_AddChildActorComponent-2` :`RelativeTransform` _output)))))

(fn `UserConstructionScript`
  (`self.SetSpawnPoints`)
  (`self.SpawnObstacle`))