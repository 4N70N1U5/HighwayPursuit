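; HealthItem is a clickable pickup actor that restores a fixed amount of health to the player's car.
; After a short delay on BeginPlay, it caches the HUD reference from MyGameMode.
; Hovering the cursor over its HeartSymbol toggles the HUD's collect banner.
; Clicking it plays a sound, adds clamped health to the PlayerCar pawn, hides the banner and destroys the item.
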(event `self.ReceiveBeginPlay`
  (`KismetSystemLibrary.Delay` 0.2)
  (bind _asmy_game_mode (cast `/Game/Blueprints/MyGameMode` (`GameplayStatics.GetGameMode`)))
  (set `self.HUDReference` (`/Game/Blueprints/MyGameMode.HUDReference` _asmy_game_mode)))

(event `self.HeartSymbol.OnBeginCursorOver`
  (params (TouchedComponent :type "PrimitiveComponent Object Reference"))
  (`Widget.SetVisibility` (`/Game/Blueprints/HUD.CollectBanner` (`self.HUDReference`)) "Visible"))

(event `self.HeartSymbol.OnEndCursorOver`
  (params (TouchedComponent :type "PrimitiveComponent Object Reference"))
  (`Widget.SetVisibility` (`/Game/Blueprints/HUD.CollectBanner` (`self.HUDReference`)) "Collapsed"))

(event `self.HeartSymbol.OnClicked`
  (params (TouchedComponent :type "PrimitiveComponent Object Reference") (ButtonPressed :type "Key Structure"))
  (`GameplayStatics.PlaySound2D` "/Game/SFX/GetHealthSFX.GetHealthSFX" 1.0 1.0 0.0 null null)
  (bind _asplayer_car (cast `/Game/Blueprints/PlayerCar` (`GameplayStatics.GetPlayerPawn` 0)))
  (set `/Game/Blueprints/PlayerCar.Health` (`KismetMathLibrary.FClamp` (+ (`/Game/Blueprints/PlayerCar.Health` _asplayer_car) 30.0) 0.0 100.0) _asplayer_car)
  (`Widget.SetVisibility` (`/Game/Blueprints/HUD.CollectBanner` (`self.HUDReference`)) "Collapsed")
  (`self.K2_DestroyActor`))

(fn `UserConstructionScript`)